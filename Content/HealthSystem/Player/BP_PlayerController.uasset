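; Player controller for the health system sample that sets game-only input on begin play and handles pausing.
; The pause input action toggles between pause and unpause events based on whether the game is paused.
; Pausing creates the pause widget, switches to game-and-UI input and shows a cursor centered in the viewport.
; Unpausing removes and clears the widget, then restores game-only input and hides the cursor.
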(event Custom|Pause%20Game
  (bind _returnvalue (Viewport|GetViewportSize))
  (bind (_x _y) (Math|Vector2D|BreakVector2D _returnvalue))
  (Game|SetGamePaused true)
  (Variables|Default|GetPause%20Widget
    (:then)
    (:else
      (bind _returnvalue_2 (UserInterface|CreateWidget "/Game/HealthSystem/Widgets+UI/WB_Pause.WB_Pause_C"))
      (bind _output_get (Variables|Default|SetPause%20Widget _returnvalue_2))
      (UserInterface|Viewport|AddtoViewport _output_get 0)
      (Input|SetInputModeGameandUI self _output_get "DoNotLock" false false)
      (Variables|Default|SetbShowMouseCursor true)
      (Class|PlayerController|SetMouseLocation (Math|Float|Truncate (* _x 0.5)) (Math|Float|Truncate (* _y 0.5))))))

(event Custom|Unpause%20Game
  (Game|SetGamePaused false)
  (bind _pause_widget (Variables|Default|GetPause%20Widget)
    (:then
      (Widget|RemovefromParent _pause_widget)
      (Variables|Default|SetPause%20Widget 0)
      (Input|SetInputModeGameOnly self false)
      (Variables|Default|SetbShowMouseCursor false))
    (:else)))

(event Input|EnhancedActionEvents|EnhancedInputActionIA_Pause
  (params (ActionValue :type Boolean) (ElapsedSeconds :type Float%20%28double-precision%29) (TriggeredSeconds :type Float%20%28double-precision%29) (InputAction :type Input%20Action%20Object%20Reference :default "/Game/HealthSystem/Player/Input/Actions/IA_Pause.IA_Pause"))
  (:Started
    (if (Game|IsGamePaused)
      (CallFunction|UnpauseGame)
      (else
        (CallFunction|PauseGame)))))

(event EventBeginPlay
  (Input|SetInputModeGameOnly (Game|GetPlayerController 0) false))

(fn ConstructionScript)