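; BP_SpawnHealthBar is an actor that attaches a floating health bar widget to a target actor.
; On BeginPlay it caches the first-person player character, adds a scaled-down widget component above ActorToAttachTo, and passes its ACHealth reference into the WB_HealthBar widget.
; Every Tick it calls FaceCamera with the widget component and player to keep the bar turned toward the player's view.
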(event EventBeginPlay
  (bind _asbp_first_person_character (Utilities|Casting|CastToBP_FirstPersonCharacter (Game|Player|GetPlayerPawn 0)))
  (Variables|Default|SetPlayer _asbp_first_person_character)
  (bind _returnvalue (AddComponent|AddWidgetComponent (Variables|Default|GetActor%20to%20attach%20to) false (Math|Transform|MakeTransform "0.000000,0.000000,100.000000" "0, 0, 0" "0.200000,0.200000,0.200000")))
  (Variables|Default|SetWidget _returnvalue)
  (bind _aswb_health_bar (Utilities|Casting|CastToWB_HealthBar (UserInterface|GetWidget _returnvalue)))
  (Variables|/Game/HealthSystem/Widgets+UI/WB_HealthBar.WB_HealthBar_C|SetAC%20Health _aswb_health_bar (Variables|Default|GetAC%20Health)))

(event EventTick
  (params (DeltaSeconds :type Float%20%28single-precision%29))
  (Utilities|FaceCamera (Variables|Default|GetWidget) (Variables|Default|GetPlayer)))

(fn ConstructionScript)