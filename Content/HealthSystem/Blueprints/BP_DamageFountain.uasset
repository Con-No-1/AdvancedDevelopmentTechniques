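; BP_DamageFountain is a damage-over-time area that hurts the local first-person player while they overlap its sphere.
; Each tick it applies DamagePerSecond scaled by frame time and horizontal distance, ramping from zero at the sphere's edge to full at half radius.
; A text label, set to the DPS value in the construction script, turns every tick to face the player's camera.
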(event EventBeginPlay
  (bind _asbp_first_person_character (Utilities|Casting|CastToBP_FirstPersonCharacter (Pawn|GetControlledPawn (Game|GetPlayerController 0))))
  (Variables|Default|SetLocal%20Player _asbp_first_person_character))

(event EventTick
  (params (DeltaSeconds :type Float%20%28single-precision%29))
  (Variables|Default|SetDelta%20Seconds DeltaSeconds)
  (Utilities|FlowControl|Sequence
    (:then_0
      (for _array_element (Collision|GetOverlappingActors (Variables|Default|GetSphere) "/Game/HealthSystem/Blueprints/BP_FirstPersonCharacter.BP_FirstPersonCharacter_C" :!class /Script/Engine.PrimitiveComponent)
        (if (== _array_element (Variables|Default|GetLocal%20Player))
          (Game|Damage|ApplyDamage (Variables|Default|GetLocal%20Player) (CallFunction|CalcDamage) 0 self))))
    (:then_1
      (Transformation|SetWorldRotation (Variables|Default|GetTextRender) (Math|Rotator|FindLookatRotation (Transformation|GetWorldLocation (Variables|Default|GetTextRender)) (Transformation|GetWorldLocation (Variables|/Game/HealthSystem/Blueprints/BP_FirstPersonCharacter.BP_FirstPersonCharacter_C|GetFirstPersonCamera (Variables|Default|GetLocal%20Player)))) false false))))

(fn ConstructionScript
  (Rendering|Components|TextRender|SetText (Variables|Default|GetTextRender) (Utilities|Text|FormatText "DPS: {x}" (Variables|Default|GetDamage%20per%20Second))))

(fn CalcDamage
  (return (* (Variables|Default|GetDelta%20Seconds) (Variables|Default|GetDamage%20per%20Second) (CallFunction|DistanceMulti))))

(fn DistanceMulti
  (bind _sphere (Variables|Default|GetSphere))
  (bind _returnvalue (Components|Sphere|GetScaledSphereRadius _sphere))
  (return (Math|Float|MapRangeClamped (Math|Vector|Distance2D(Vector) (Transformation|GetActorLocation) (Transformation|GetActorLocation (Variables|Default|GetLocal%20Player))) _returnvalue (/ _returnvalue 2.0) 0.0 1.0)))