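; AC_Health is an actor component that tracks health for its owner, with events for healing, damage and revival.
; Heal and Damage clamp CurrentHealth between zero and MaxHealth, while Revive restores it to full and calls Revived.
; CurrentHealth uses a RepNotify that calls HealthUpdated on each notify and Death at zero or below.
; BeginPlay also calls HealthUpdated to broadcast the starting state.
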(event Custom|Revive
  (Variables|Default|SetCurrent%20Health (Variables|Default|GetMax%20Health))
  (Default|CallRevived))

(event Custom|Heal
  (params (Heal%20Amount :type Float%20%28double-precision%29))
  (Variables|Default|SetCurrent%20Health (Math|Float|Clamp(Float) (+ (Variables|Default|GetCurrent%20Health) Heal%20Amount) 0.0 (Variables|Default|GetMax%20Health))))

(event Custom|Damage
  (params (Damage%20Amount :type Float%20%28double-precision%29))
  (Variables|Default|SetCurrent%20Health (Math|Float|Clamp(Float) (- (Variables|Default|GetCurrent%20Health) Damage%20Amount) 0.0 (Variables|Default|GetMax%20Health))))

(event EventBeginPlay
  (Default|CallHealthUpdated))

(fn OnRepCurrentHealth
  (Default|CallHealthUpdated)
  (if (<= (Variables|Default|GetCurrent%20Health) 0.0)
    (Default|CallDeath)))