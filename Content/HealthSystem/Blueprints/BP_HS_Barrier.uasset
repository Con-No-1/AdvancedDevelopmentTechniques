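; BP_HS_Barrier is a health system trigger barrier that sets the first-person character's health and bottles when they pass through it.
; On overlap, it writes current health to the character's ACHealth component, calls RemoveBottle, adds the configured bottles, and can enable a blocker against backtracking.
; The construction script sizes trigger and blocker boxes from Width, and Tick turns the level text toward the player.
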(event OnComponentBeginOverlap(Overlap)
  (params (OverlappedComponent :type Primitive%20Component%20Object%20Reference) (OtherActor :type Actor%20Object%20Reference) (OtherComp :type Primitive%20Component%20Object%20Reference) (OtherBodyIndex :type Integer) (bFromSweep :type Boolean) (SweepResult :type Hit%20Result%20Structure%20%28by%20ref%29))
  (bind _blocker (Variables|Default|GetBlocker))
  (bind _asbp_first_person_character (Utilities|Casting|CastToBP_FirstPersonCharacter OtherActor))
  (if (Variables|Default|GetDo%20Once)
    (Utilities|FlowControl|DoOnce false
      (:Completed
        _)))
  (Utilities|FlowControl|Sequence
    (:then_0
      (Variables|/Game/HealthSystem/Blueprints/AC_HealthSystem.AC_HealthSystem_C|SetCurrent%20Health (Variables|/Game/HealthSystem/Blueprints/BP_FirstPersonCharacter.BP_FirstPersonCharacter_C|GetAC_Health _asbp_first_person_character) (Variables|Default|GetHealth)))
    (:then_1
      (Default|RemoveBottle (Variables|/Game/HealthSystem/Blueprints/BP_FirstPersonCharacter.BP_FirstPersonCharacter_C|GetAC_Health _asbp_first_person_character) true)
      (for _index (range 1 (Variables|Default|GetBottles))
        (Default|AddBottle (Variables|/Game/HealthSystem/Blueprints/BP_FirstPersonCharacter.BP_FirstPersonCharacter_C|GetAC_Health _asbp_first_person_character) (Variables|Default|GetBottle%20Health))))
    (:then_2
      (if (Variables|Default|GetBacktrack%20Blocker)
        (Collision|SetCollisionEnabled _blocker "QueryAndPhysics")
        (Collision|SetCollisionResponsetoAllChannels _blocker "ECR_Block")))))

(event EventBeginPlay
  (bind _asbp_first_person_character (Utilities|Casting|CastToBP_FirstPersonCharacter (Game|Player|GetPlayerPawn 0)))
  (Variables|Default|SetLocal%20Player _asbp_first_person_character))

(event Collision|EventActorBeginOverlap
  (params (OtherActor :type Actor%20Object%20Reference)))

(event EventTick
  (params (DeltaSeconds :type Float%20%28single-precision%29))
  (bind _level_text (Variables|Default|GetLevel%20Text)
    (:then
      (Utilities|FaceCamera _level_text (Variables|Default|GetLocal%20Player)))
    (:else)))

(fn ConstructionScript
  (bind _width (Variables|Default|GetWidth))
  (Components|Box|SetBoxExtent (Variables|Default|GetOverlap) (Math|Vector|MakeVector 12.5 _width 2.5e+02) true)
  (Components|Box|SetBoxExtent (Variables|Default|GetBlocker) (Math|Vector|MakeVector 25.0 _width 2.5e+02) true))