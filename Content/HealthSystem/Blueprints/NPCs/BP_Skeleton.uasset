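; Skeleton NPC that fights other skeletons, with an Enemy flag setting gear materials, health and player targeting rules.
; A looping timer plays melee attacks and damages the target in range, while a delayed AIMoveTo loop pursues it.
; SelectTarget picks a random living skeleton without checking team, pairing mutually if that one lacks a target.
; AC_Health events drive the material's health and hit flash, health bar visibility, death stop and revive montage.
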(event HealthUpdated(AC_Health)
  (bind _ac_health (Variables|Default|GetAC_Health))
  (Rendering|Material|SetScalarParameterValue (Variables|Default|GetMaterial) "Health" (/ (Variables|/Game/HealthSystem/Blueprints/AC_Health.AC_Health_C|GetCurrent%20Health _ac_health) (Variables|/Game/HealthSystem/Blueprints/AC_Health.AC_Health_C|GetMax%20Health _ac_health)) :!class /Script/Engine.MaterialInstanceDynamic)
  (Rendering|Material|SetScalarParameterValue (Variables|Default|GetMaterial) "Emissive" 0.25 :!class /Script/Engine.MaterialInstanceDynamic)
  (Utilities|FlowControl|RetriggerableDelay 0.1)
  (Rendering|Material|SetScalarParameterValue (Variables|Default|GetMaterial) "Emissive" 0.0 :!class /Script/Engine.MaterialInstanceDynamic))

(event Death(AC_Health)
  (Variables|Default|SetCan%20Fight false)
  (Components|Movement|StopMovementImmediately (Variables|Character|GetCharacterMovement))
  (Rendering|SetVisibility (Variables|Default|GetHealth%20Bar) false false)
  (Animation|StopAnimMontage (Animation|GetCurrentMontage :!class /Script/Engine.Character)))

(event Revived(AC_Health)
  (bind _returnvalue (Animation|PlayAnimMontage "/Game/HealthSystem/Mesh+Mats/Skeleton/Animations/AM_SkeletonRevive.AM_SkeletonRevive" 1.0 "None"))
  (Utilities|FlowControl|Delay _returnvalue)
  (Variables|Default|SetCan%20Fight true)
  (Rendering|SetVisibility (Variables|Default|GetHealth%20Bar) true false))

(event Custom|Wander
  (if (Variables|/Game/HealthSystem/Blueprints/AC_Health.AC_Health_C|GetAlive (Variables|Default|GetAC_Health)) :!label _label
    (AI|AIMoveTo self (.RandomLocation (AI|Navigation|GetRandomReachablePointinRadius (Transformation|GetActorLocation) 1e+03 0 0)) 0 5.0 false
      (:OnSuccess
        _)
      (:OnFail
        _))
    (Utilities|FlowControl|Delay (Math|Random|RandomFloatinRange 1.0 5.0))
    (goto _label)))

(event Custom|Walk%20to%20Target
  (bind _target_skeleton (Variables|Default|GetTarget%20Skeleton :!label _label)
    (:then
      (AI|AIMoveTo self "0, 0, 0" _target_skeleton 1.5e+02 false
        (:OnSuccess
          _)
        (:OnFail
          _))
      (Utilities|FlowControl|Delay (Math|Random|RandomFloatinRange 1.0 5.0))
      (goto _label))
    (:else
      (Utilities|FlowControl|DelayUntilNextTick)
      (CallFunction|SelectTarget)
      (goto _label))))

(event Custom|Attack
  (if (Variables|Default|GetCan%20Fight)
    (bind _target_skeleton (Variables|Default|GetTarget%20Skeleton)
      (:then
        (if (and (< (Transformation|GetDistanceTo _target_skeleton) 2e+02) (Variables|BP_Skeleton_C|GetCan%20Fight _target_skeleton))
          (Animation|PlayAnimMontage "/Game/HealthSystem/Mesh+Mats/Skeleton/Animations/AM_SkeletonAttack.AM_SkeletonAttack" 1.0 "None")
          (Utilities|FlowControl|Delay 0.4)
          (if (Variables|/Game/HealthSystem/Blueprints/AC_Health.AC_Health_C|GetAlive (Variables|Default|GetAC_Health))
            (Default|Damage (Variables|BP_Skeleton_C|GetAC_Health (Variables|Default|GetTarget%20Skeleton)) (Math|Random|RandomFloatinRange 5.0 1e+01)))))
      (:else))))

(event EventBeginPlay
  (bind _asbp_first_person_character (Utilities|Casting|CastToBP_FirstPersonCharacter (Game|Player|GetPlayerPawn 0)))
  (Variables|Default|SetPlayer _asbp_first_person_character)
  (bind _aswb_health_bar (Utilities|Casting|CastToWB_HealthBar (UserInterface|GetWidget (Variables|Default|GetHealth%20Bar))))
  (Variables|/Game/HealthSystem/Widgets+UI/WB_HealthBar.WB_HealthBar_C|SetAC%20Health _aswb_health_bar (Variables|Default|GetAC_Health))
  (Utilities|Time|SetTimerbyEvent (delegate Custom|Attack) 1.5 true true 0.0 1.5)
  (Utilities|FlowControl|Delay 0.2)
  (CallFunction|WalktoTarget))

(event EventTick
  (params (DeltaSeconds :type Float%20%28single-precision%29))
  (Utilities|FaceCamera (Variables|Default|GetHealth%20Bar) (Variables|Default|GetPlayer)))

(fn ConstructionScript
  (bind _ac_health (Variables|Default|GetAC_Health))
  (bind _ac_health_2 (Variables|Default|GetAC_Health))
  (Utilities|FlowControl|Sequence
    (:then_0
      (bind _returnvalue (Rendering|Material|CreateDynamicMaterialInstance "/Game/HealthSystem/Mesh+Mats/Skeleton/M_Skeleton.M_Skeleton" "None" "None" :!class /Script/Engine.KismetMaterialLibrary))
      (bind _output_get (Variables|Default|SetMaterial _returnvalue))
      (Rendering|Material|SetMaterial (Variables|Character|GetMesh) 0 _output_get))
    (:then_1
      (Rendering|Material|SetMaterial (Variables|Character|GetMesh) 1 (select (Variables|Default|GetEnemy) "/Game/HealthSystem/Mesh+Mats/Skeleton/M_ShieldE.M_ShieldE" "/Game/HealthSystem/Mesh+Mats/Skeleton/M_ShieldF.M_ShieldF"))
      (Rendering|Material|SetMaterial (Variables|Character|GetMesh) 2 (select (Variables|Default|GetEnemy) "/Game/HealthSystem/Mesh+Mats/Skeleton/M_SwordE.M_SwordE" "/Game/HealthSystem/Mesh+Mats/Skeleton/M_SwordF.M_SwordF")))
    (:then_2
      (if (Variables|Default|GetEnemy)
        (Variables|/Game/HealthSystem/Blueprints/AC_Health.AC_Health_C|SetPlayer%20can%20Target (Variables|Default|GetAC_Health) false)
        (bind _output_get_2 (Variables|/Game/HealthSystem/Blueprints/AC_Health.AC_Health_C|SetMax%20Health _ac_health_2 2e+02))
        (Variables|/Game/HealthSystem/Blueprints/AC_Health.AC_Health_C|SetCurrent%20Health _ac_health_2 _output_get_2)
        (else
          (Variables|/Game/HealthSystem/Blueprints/AC_Health.AC_Health_C|SetPlayer%20can%20Target (Variables|Default|GetAC_Health) true)
          (Variables|/Game/HealthSystem/Blueprints/AC_Health.AC_Health_C|SetPlayer%20can%20Damage (Variables|Default|GetAC_Health) false)
          (bind _output_get_3 (Variables|/Game/HealthSystem/Blueprints/AC_Health.AC_Health_C|SetMax%20Health _ac_health 1e+02))
          (Variables|/Game/HealthSystem/Blueprints/AC_Health.AC_Health_C|SetCurrent%20Health _ac_health _output_get_3))))))

(fn SelectTarget
  (bind _target_skeleton (Variables|Default|GetTarget%20Skeleton)
    (:then
      (if (not (Variables|/Game/HealthSystem/Blueprints/AC_Health.AC_Health_C|GetAlive (Variables|BP_Skeleton_C|GetAC_Health _target_skeleton)))
        (bind _outactors (Actor|GetAllActorsOfClass "BP_Skeleton_C" :!label _label))
        (bind _output_get (LocalVariables|SetSkeletons _outactors))
        (Utilities|Array|Shuffle _output_get)
        (bind _array_element (Utilities|Array|ForEachLoopwithBreak (LocalVariables|GetSkeletons) :!label _label_2)
          (:LoopBody
            (if (Variables|/Game/HealthSystem/Blueprints/AC_Health.AC_Health_C|GetAlive (Variables|BP_Skeleton_C|GetAC_Health _array_element))
              (Variables|BP_Skeleton_C|GetTarget%20Skeleton _array_element
                (:then
                  _)
                (:else
                  (Variables|BP_Skeleton_C|SetTarget%20Skeleton _array_element self)))
              (Variables|Default|SetTarget%20Skeleton _array_element)
              (goto _label_2 Break)))
          (:Completed
            (CallFunction|WalktoTarget)))))
    (:else
      (goto _label))))