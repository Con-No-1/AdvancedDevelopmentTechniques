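; Actor component that manages health, death and revival, backed by reserve health bottles stored as one fractional fill count.
; Damage lowers health, Heal overflows into bottles, and reaching zero consumes a bottle or kills the owner.
; RepNotify functions compare previous values to fire health, bottle and life-state events.
; It optionally spawns a health bar actor, and adding or removing bottles edits vial widgets on a first-person character's HUD.
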(event Custom|Set%20Bottle%20Consumed%20this%20tick
  (Variables|Default|SetBottle%20Consumed%20this%20tick true)
  (Utilities|FlowControl|DelayUntilNextTick)
  (Variables|Default|SetBottle%20Consumed%20this%20tick false))

(event EventBeginPlay
  (Utilities|FlowControl|Sequence
    (:then_0
      (bind _asbp_first_person_character (Utilities|Casting|CastToBP_FirstPersonCharacter (Game|Player|GetPlayerPawn 0)))
      (Variables|Default|SetLocal%20Player _asbp_first_person_character)
      (Variables|Default|Set_prevCurrent%20Health (Variables|Default|GetCurrent%20Health))
      (Variables|Default|Set_prevBottlesFilled%25 (Variables|Default|GetBottles%20Filled%20%25)))
    (:then_1
      (if (<= (Variables|Default|GetCurrent%20Health) 0.0)
        (CallFunction|HealthReached0)))
    (:then_2
      (Utilities|FlowControl|DelayUntilNextTick)
      (Default|CallHealthUpdated)
      (if (Variables|Default|GetSpawn%20Health%20Bar%20Widget)
        (Game|SpawnActorfromClass "/Game/HealthSystem/Widgets+UI/BP_SpawnHealthBar.BP_SpawnHealthBar_C" (Math|Transform|MakeTransform "0, 0, 0" "0, 0, 0" "1.000000,1.000000,1.000000") "Undefined" "MultiplyWithRoot" 0 self (Components|GetOwner) 0)))))

(fn OnRepCurrentHealth
  (if (!= (Variables|Default|GetCurrent%20Health) (Variables|Default|Get_prevCurrent%20Health))
    (Utilities|FlowControl|Sequence
      (:then_0
        (Utilities|FlowControl|Sequence
          (:then_0
            (if (Variables|Default|GetAlive)
              (if (<= (Variables|Default|GetCurrent%20Health) 0.0)
                (CallFunction|HealthReached0))
              (elif (> (Variables|Default|GetCurrent%20Health) 0.0)
                (Variables|Default|SetAlive true))))
          (:then_1
            (Default|CallHealthUpdated))
          (:then_2
            (if (> (Variables|Default|GetCurrent%20Health) (Variables|Default|Get_prevCurrent%20Health))
              (Default|CallHealthIncreased)
              (else
                (Default|CallHealthDecreased))))
          (:then_3
            (if (>= (Variables|Default|GetCurrent%20Health) (Variables|Default|GetMax%20Health))
              (if (not (Variables|Default|GetBottle%20Consumed%20this%20tick))
                (Default|CallHealthFilled))))))
      (:then_1
        (Variables|Default|Set_prevCurrent%20Health (Variables|Default|GetCurrent%20Health))))))

(fn OnRepBottlesFilled%
  (if (!= (Variables|Default|GetBottles%20Filled%20%25) (Variables|Default|Get_prevBottlesFilled%25))
    (Utilities|FlowControl|Sequence
      (:then_0
        (Default|CallBottle%Updated))
      (:then_1
        (if (> (Variables|Default|GetBottles%20Filled%20%25) (Variables|Default|Get_prevBottlesFilled%25))
          (Default|CallBottle%Increased)
          (if (> (Math|Float|Floor (Variables|Default|GetBottles%20Filled%20%25)) (Variables|Default|Get_prevBottlesFilled%25))
            (Default|CallBottleFilled)
            (if (>= (Variables|Default|GetBottles%20Filled%20%25) (.Max%20Bottle%20%25 (CallFunction|BottleStats)))
              (Default|CallAllBottlesFilled)))
          (else
            (Default|CallBottle%Decreased)))))))

(fn OnRepAlive
  (if (Variables|Default|GetAlive)
    (Default|CallRevived)
    (else
      (Default|CallDeath))))

(fn BottleStats
  (return (Math|Conversions|ToFloat(Integer) (Variables|Default|GetBottles)) (* (Variables|Default|GetMax%20Health) (Variables|Default|GetBottles%20Filled%20%25)) (* (Variables|Default|GetMax%20Health) (Math|Conversions|ToFloat(Integer) (Variables|Default|GetBottles))) (+ (* (Variables|Default|GetMax%20Health) (Variables|Default|GetBottles%20Filled%20%25)) (Variables|Default|GetCurrent%20Health)) (+ (* (Variables|Default|GetMax%20Health) (Math|Conversions|ToFloat(Integer) (Variables|Default|GetBottles))) (Variables|Default|GetMax%20Health))))

(fn Damage
  (params (Damage :type Float%20%28double-precision%29))
  (if (Variables|Default|GetCan%20be%20Damaged)
    (LocalVariables|SetHealth (Variables|Default|GetCurrent%20Health))
    (Variables|Default|SetCurrent%20Health (Math|Float|Clamp(Float) (- (LocalVariables|GetHealth) (Math|Float|Clamp(Float) Damage 0.0 (LocalVariables|GetHealth))) 0.0 (Variables|Default|GetMax%20Health)))
    (return (Math|Float|Clamp(Float) Damage 0.0 (LocalVariables|GetHealth)))
    (else
      (return 0.0))))

(fn HealthReached0
  (if (> (Variables|Default|GetBottles%20Filled%20%25) 0.0)
    (CallFunction|ConsumeBottle)
    (else
      (Variables|Default|SetAlive false))))

(fn Heal
  (params (Heal :type Float%20%28double-precision%29))
  (bind (_max_bottle__ _current_bottle_health _max_bottle_health) (CallFunction|BottleStats))
  (bind (_max_bottle___2 _current_bottle_health_2 _max_bottle_health_2) (CallFunction|BottleStats))
  (LocalVariables|SetStart%20Health (Variables|Default|GetCurrent%20Health))
  (LocalVariables|SetStart%20Bottle%20Health (.Current%20Bottle%20Health (CallFunction|BottleStats)))
  (LocalVariables|SetHeal%20Remaining Heal)
  (if (and (Variables|Default|GetCan%20be%20Healed) (or (Variables|Default|GetAlive) (Variables|Default|GetCan%20be%20Revived)))
    (LocalVariables|SetHealth (Variables|Default|GetCurrent%20Health))
    (Utilities|FlowControl|Sequence
      (:then_0
        (Variables|Default|SetCurrent%20Health (Math|Float|Clamp(Float) (+ Heal (Variables|Default|GetCurrent%20Health)) 0.0 (Variables|Default|GetMax%20Health)))
        (LocalVariables|SetHeal%20Remaining (- (LocalVariables|GetHeal%20Remaining) (- (Variables|Default|GetCurrent%20Health) (LocalVariables|GetStart%20Health)))))
      (:then_1
        (if (> (LocalVariables|GetHeal%20Remaining) 0.0)
          (if (< _current_bottle_health_2 _max_bottle_health_2)
            (Variables|Default|SetBottles%20Filled%20%25 (/ (+ (.Current%20Bottle%20Health (CallFunction|BottleStats)) (Math|Float|Clamp(Float) (LocalVariables|GetHeal%20Remaining) 0.0 (Math|Float|Absolute(Float) (- _current_bottle_health _max_bottle_health)))) (Variables|Default|GetMax%20Health)))
            (LocalVariables|SetHeal%20Remaining (- (LocalVariables|GetHeal%20Remaining) (- (.Current%20Bottle%20Health (CallFunction|BottleStats)) (LocalVariables|GetStart%20Bottle%20Health)))))))
      (:then_2
        (return (- Heal (LocalVariables|GetHeal%20Remaining)))))
    (else
      (return 0.0))))

(fn Revive
  (if (Variables|Default|GetCan%20be%20Revived)
    (if (<= (Variables|Default|GetCurrent%20Health) (Variables|Default|GetMax%20Health))
      (Variables|Default|SetCurrent%20Health (Variables|Default|GetMax%20Health)))))

(fn AddBottle
  (params (Fullness :type Float%20%28double-precision%29))
  (Utilities|FlowControl|Sequence
    (:then_0
      (Math|Integer|IncrementInt (Variables|Default|GetBottles)
        (:%20%20
          (Variables|Default|SetBottles%20Filled%20%25 (Math|Float|Clamp(Float) (+ (Variables|Default|GetBottles%20Filled%20%25) Fullness) 0.0 (Math|Conversions|ToFloat(Integer) (Variables|Default|GetBottles))))
          (if (and (<= (Variables|Default|GetCurrent%20Health) 0.0) (> (Variables|Default|GetBottles%20Filled%20%25) 0.0))
            (CallFunction|ConsumeBottle)
            (CallFunction|Revive)))))
    (:then_1
      (bind _asbp_first_person_character (Utilities|Casting|CastToBP_FirstPersonCharacter (Components|GetOwner)))
      (bind _returnvalue (UserInterface|CreateWidget "/Game/HealthSystem/Widgets+UI/WB_Vial.WB_Vial_C" 0 (Variables|Default|GetBottles) (Variables|/Game/HealthSystem/Blueprints/BP_FirstPersonCharacter.BP_FirstPersonCharacter_C|GetAC_Health _asbp_first_person_character)))
      (Widget|Panel|AddChild (Variables|/Game/HealthSystem/Widgets+UI/WB_HealthSystemUI.WB_HealthSystemUI_C|GetVialBox (Variables|/Game/HealthSystem/Blueprints/BP_FirstPersonCharacter.BP_FirstPersonCharacter_C|GetHealth%20UI _asbp_first_person_character)) _returnvalue))
    (:then_2
      (Default|CallBottleAdded))))

(fn ConsumeBottle
  (CallFunction|SetBottleConsumedThisTick)
  (Utilities|FlowControl|Sequence
    (:then_0
      (if (< (Variables|Default|GetBottles%20Filled%20%25) 1.0)
        (Variables|Default|SetCurrent%20Health (* (Variables|Default|GetMax%20Health) (Variables|Default|GetBottles%20Filled%20%25)))
        (Variables|Default|SetBottles%20Filled%20%25 0.0)
        (else
          (Variables|Default|SetCurrent%20Health (Variables|Default|GetMax%20Health))
          (Variables|Default|SetBottles%20Filled%20%25 (- (Variables|Default|GetBottles%20Filled%20%25) 1.0)))))
    (:then_1
      (Default|CallBottleConsumed))))

(fn RemoveBottle
  (if (> (Variables|Default|GetBottles) 0)
    (Utilities|FlowControl|Sequence
      (:then_0
        (Math|Integer|DecrementInt (Variables|Default|GetBottles)
          (:%20%20
            (LocalVariables|Set_Bottle%20%25 (Math|Float|Clamp(Float) (Variables|Default|GetBottles%20Filled%20%25)))
            (Variables|Default|SetBottles%20Filled%20%25 (Math|Float|Clamp(Float) (- (Variables|Default|GetBottles%20Filled%20%25) 1.0) 0.0 (Math|Conversions|ToFloat(Integer) (Variables|Default|GetBottles)))))))
      (:then_1
        (bind _asbp_first_person_character (Utilities|Casting|CastToBP_FirstPersonCharacter (Components|GetOwner)))
        (bind _array_element (Utilities|Array|ForEachLoopwithBreak (Class|PanelWidget|GetAllChildren (Variables|/Game/HealthSystem/Widgets+UI/WB_HealthSystemUI.WB_HealthSystemUI_C|GetVialBox (Variables|/Game/HealthSystem/Blueprints/BP_FirstPersonCharacter.BP_FirstPersonCharacter_C|GetHealth%20UI _asbp_first_person_character))))
          (:Completed
            (Widget|RemovefromParent _array_element))))
      (:then_2
        (Default|CallBottleRemoved)
        (return (LocalVariables|Get_Bottle%20%25))))))