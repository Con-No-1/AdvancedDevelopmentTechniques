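; Health component that manages damage, healing, death and revival, with refillable vials acting as reserve health bars.
; RepNotifies on CurrentHealth and Alive drive the update, death and revive calls; at zero health a vial is consumed before death.
; Heal fills vials when health is full, or empty if ReviveRequiresPotion is set.
; It optionally spawns an attached health bar actor, and AddVial adds vial widgets to the first-person character's UI.
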(event EventBeginPlay
  (Utilities|FlowControl|Sequence
    (:then_0
      (bind _asbp_first_person_character (Utilities|Casting|CastToBP_FirstPersonCharacter (Game|Player|GetPlayerPawn 0)))
      (Variables|Default|SetLocal%20Player _asbp_first_person_character))
    (:then_1
      (if (<= (Variables|Default|GetCurrent%20Health) 0.0)
        (CallFunction|HealthReached0)))
    (:then_2
      (Utilities|FlowControl|DelayUntilNextTick)
      (Default|CallHealthUpdated)
      (if (Variables|Default|GetSpawn%20Health%20Bar%20Widget)
        (Game|SpawnActorfromClass "/Game/HealthSystem/Widgets+UI/BP_SpawnHealthBar.BP_SpawnHealthBar_C" (Math|Transform|MakeTransform "0, 0, 0" "0, 0, 0" "1.000000,1.000000,1.000000") "Undefined" "MultiplyWithRoot" 0 self (Components|GetOwner) 0)))))

(fn OnRepCurrentHealth
  (if (!= (Variables|Default|GetCurrent%20Health) (Variables|Default|Get_prevCurrent%20Health))
    (Utilities|FlowControl|Sequence
      (:then_0
        (Default|CallHealthUpdated)
        (if (Variables|Default|GetAlive)
          (if (<= (Variables|Default|GetCurrent%20Health) 0.0)
            (CallFunction|HealthReached0))
          (elif (> (Variables|Default|GetCurrent%20Health) 0.0)
            (Variables|Default|SetAlive true))))
      (:then_1
        (Variables|Default|Set_prevCurrent%20Health (Variables|Default|GetCurrent%20Health))))))

(fn VialStats
  (return (Math|Conversions|ToFloat(Integer) (Variables|Default|GetVials)) (* (Variables|Default|GetMax%20Health) (Variables|Default|GetVials%20Filled%20%25)) (* (Variables|Default|GetMax%20Health) (Math|Conversions|ToFloat(Integer) (Variables|Default|GetVials))) (+ (* (Variables|Default|GetMax%20Health) (Variables|Default|GetVials%20Filled%20%25)) (Variables|Default|GetCurrent%20Health)) (+ (* (Variables|Default|GetMax%20Health) (Math|Conversions|ToFloat(Integer) (Variables|Default|GetVials))) (Variables|Default|GetMax%20Health))))

(fn Damage
  (params (Damage :type Float%20%28double-precision%29))
  (if (Variables|Default|GetCan%20be%20Damaged)
    (LocalVariables|SetHealth (Variables|Default|GetCurrent%20Health))
    (Variables|Default|SetCurrent%20Health (Math|Float|Clamp(Float) (- (LocalVariables|GetHealth) (Math|Float|Clamp(Float) Damage 0.0 (LocalVariables|GetHealth))) 0.0 (Variables|Default|GetMax%20Health)))
    (return (Math|Float|Clamp(Float) Damage 0.0 (LocalVariables|GetHealth)))
    (else
      (return 0.0))))

(fn HealthReached0
  (if (> (Variables|Default|GetVials%20Filled%20%25) 0.0)
    (CallFunction|ConsumeVial)
    (else
      (Variables|Default|SetAlive false))))

(fn Heal
  (params (Heal :type Float%20%28double-precision%29))
  (bind (_max_vial__ _vial_health _max_vial_health) (CallFunction|VialStats))
  (if (and (Variables|Default|GetCan%20be%20Healed) (or (Variables|Default|GetAlive) (Variables|Default|GetCan%20be%20Revived)))
    (LocalVariables|SetHealth (Variables|Default|GetCurrent%20Health))
    (if (and (select (Variables|Default|GetRevive%20Requires%20Potion) (> (LocalVariables|GetHealth) 0.0) true) (< (LocalVariables|GetHealth) (Variables|Default|GetMax%20Health)))
      (Variables|Default|SetCurrent%20Health (+ (LocalVariables|GetHealth) (Math|Float|Clamp(Float) Heal 0.0 (Math|Float|Absolute(Float) (- (LocalVariables|GetHealth) (Variables|Default|GetMax%20Health))))))
      (return (Math|Float|Clamp(Float) Heal 0.0 (Math|Float|Absolute(Float) (- (LocalVariables|GetHealth) (Variables|Default|GetMax%20Health)))))
      (elif (< _vial_health _max_vial_health)
        (LocalVariables|SetVial%20Health (.Vial%20Health (CallFunction|VialStats)))
        (Variables|Default|SetVials%20Filled%20%25 (/ (+ (LocalVariables|GetVial%20Health) (Math|Float|Clamp(Float) Heal 0.0 (Math|Float|Absolute(Float) (- (LocalVariables|GetVial%20Health) (.Max%20Vial%20Health (CallFunction|VialStats)))))) (Variables|Default|GetMax%20Health)))
        (return (Math|Float|Clamp(Float) Heal 0.0 (Math|Float|Absolute(Float) (- (LocalVariables|GetVial%20Health) (.Max%20Vial%20Health (CallFunction|VialStats))))))
        (else
          (return 0.0))))
    (else
      (return 0.0))))

(fn Revive
  (if (Variables|Default|GetCan%20be%20Revived)
    (if (<= (Variables|Default|GetCurrent%20Health) (Variables|Default|GetMax%20Health))
      (Variables|Default|SetCurrent%20Health (Variables|Default|GetMax%20Health)))))

(fn AddVial
  (params (is%20Empty :type Boolean))
  (LocalVariables|SetEmpty is%20Empty)
  (Utilities|FlowControl|Sequence
    (:then_0
      (Math|Integer|IncrementInt (Variables|Default|GetVials)
        (:%20%20
          (Variables|Default|SetVials%20Filled%20%25 (select (LocalVariables|GetEmpty) (Variables|Default|GetVials%20Filled%20%25) (+ (Variables|Default|GetVials%20Filled%20%25) 1.0)))
          (if (and (<= (Variables|Default|GetCurrent%20Health) 0.0) (> (Variables|Default|GetVials%20Filled%20%25) 0.0))
            (CallFunction|ConsumeVial)
            (CallFunction|Revive)))))
    (:then_1
      (bind _asbp_first_person_character (Utilities|Casting|CastToBP_FirstPersonCharacter (Components|GetOwner)))
      (bind _returnvalue (UserInterface|CreateWidget "/Game/HealthSystem/Widgets+UI/WB_Vial.WB_Vial_C" 0 (Variables|Default|GetVials) (Variables|/Game/HealthSystem/Blueprints/BP_FirstPersonCharacter.BP_FirstPersonCharacter_C|GetAC_Health _asbp_first_person_character)))
      (Widget|Panel|AddChild (Variables|/Game/HealthSystem/Widgets+UI/WB_HealthSystemUI.WB_HealthSystemUI_C|GetVialBox (Variables|/Game/HealthSystem/Blueprints/BP_FirstPersonCharacter.BP_FirstPersonCharacter_C|GetHealth%20UI _asbp_first_person_character)) _returnvalue))
    (:then_2
      (Default|CallVialAdded))))

(fn ConsumeVial
  (Utilities|FlowControl|Sequence
    (:then_0
      (if (< (Variables|Default|GetVials%20Filled%20%25) 1.0)
        (Variables|Default|SetCurrent%20Health (* (Variables|Default|GetMax%20Health) (Variables|Default|GetVials%20Filled%20%25)))
        (Variables|Default|SetVials%20Filled%20%25 0.0)
        (else
          (Variables|Default|SetCurrent%20Health (Variables|Default|GetMax%20Health))
          (Variables|Default|SetVials%20Filled%20%25 (- (Variables|Default|GetVials%20Filled%20%25) 1.0)))))
    (:then_1
      (Default|CallVialConsumed))))

(fn OnRepAlive
  (if (Variables|Default|GetAlive)
    (Default|CallRevived)
    (else
      (Default|CallDeath))))