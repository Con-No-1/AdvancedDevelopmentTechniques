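; BP_NextLevel is a level transition trigger that opens another level when the first-person character walks into it.
; Its Overlap box is sized in the construction script from a Width variable, with fixed depth and height.
; On overlap by a BP_FirstPersonCharacter, it opens the referenced Level if that reference is valid.
; Each tick it calls FaceCamera to turn LevelText toward the player pawn cached at BeginPlay.
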(event OnComponentBeginOverlap(Overlap)
  (params (OverlappedComponent :type Primitive%20Component%20Object%20Reference) (OtherActor :type Actor%20Object%20Reference) (OtherComp :type Primitive%20Component%20Object%20Reference) (OtherBodyIndex :type Integer) (bFromSweep :type Boolean) (SweepResult :type Hit%20Result%20Structure%20%28by%20ref%29))
  (Utilities|Casting|CastToBP_FirstPersonCharacter OtherActor)
  (bind _level (Variables|Default|GetLevel)
    (:then
      (Game|OpenLevel(byObjectReference) _level))
    (:else)))

(event EventBeginPlay
  (bind _asbp_first_person_character (Utilities|Casting|CastToBP_FirstPersonCharacter (Game|Player|GetPlayerPawn 0)))
  (Variables|Default|SetLocal%20Player _asbp_first_person_character))

(event Collision|EventActorBeginOverlap
  (params (OtherActor :type Actor%20Object%20Reference)))

(event EventTick
  (params (DeltaSeconds :type Float%20%28single-precision%29))
  (Utilities|FaceCamera (Variables|Default|GetLevel%20Text) (Variables|Default|GetLocal%20Player)))

(fn ConstructionScript
  (Components|Box|SetBoxExtent (Variables|Default|GetOverlap) (Math|Vector|MakeVector 5e+01 (Variables|Default|GetWidth) 2.5e+02) true))