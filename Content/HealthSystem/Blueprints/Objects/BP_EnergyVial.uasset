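; BP_EnergyVial is a health pickup that heals an overlapping actor through its AC_Health component, then destroys itself.
; Collection requires that the component allows potion pickup and is below maximum health; the first-person character also gets a popup.
; The construction script scales the bottle material's fill and point light intensity from HealAmount.
; BeginPlay randomises phase and rate of the bob, wobble and spin timelines so vials move out of sync.
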(event OnComponentBeginOverlap(Collision)
  (params (OverlappedComponent :type Primitive%20Component%20Object%20Reference) (OtherActor :type Actor%20Object%20Reference) (OtherComp :type Primitive%20Component%20Object%20Reference) (OtherBodyIndex :type Integer) (bFromSweep :type Boolean) (SweepResult :type Hit%20Result%20Structure%20%28by%20ref%29))
  (bind _returnvalue (Actor|GetComponentbyClass OtherActor "/Game/HealthSystem/Blueprints/AC_Health.AC_Health_C"))
  (bind (_max_bottle__ _current_bottle_health _max_bottle_health _total_current_health _total_max_health) (Default|BottleStats _returnvalue))
  (Utilities|IsValid _returnvalue
    (:Is%20Valid
      (if (and (Variables|/Game/HealthSystem/Blueprints/AC_Health.AC_Health_C|GetCan%20collect%20Potions _returnvalue) (< _total_current_health _total_max_health))
        (Default|Heal _returnvalue (Variables|Default|GetHeal%20Amount))
        (Utilities|FlowControl|Sequence
          (:then_0
            (bind _asbp_first_person_character (Utilities|Casting|CastToBP_FirstPersonCharacter OtherActor))
            (Default|PopupText _asbp_first_person_character "Used Energy Vial"))
          (:then_1
            (Actor|DestroyActor)))))))

(event EventBeginPlay
  (bind _wobble_tl (Variables|Default|GetWobble%20TL))
  (bind _rotation_tl (Variables|Default|GetRotation%20TL))
  (bind _bob_tl (Variables|Default|GetBob%20TL))
  (Utilities|FlowControl|Sequence
    (:then_0
      (Components|Timeline|SetPlaybackPosition _bob_tl (Math|Random|RandomFloatinRange 0.0 (Components|Timeline|GetTimelineLength _bob_tl)) false true)
      (Components|Timeline|SetPlayRate (Variables|Default|GetBob%20TL) (Math|Random|RandomFloatinRange 0.2 0.4)))
    (:then_1
      (Components|Timeline|SetPlaybackPosition _wobble_tl (Math|Random|RandomFloatinRange 0.0 (Components|Timeline|GetTimelineLength _wobble_tl)) false true)
      (Components|Timeline|SetPlayRate (Variables|Default|GetWobble%20TL) (Math|Random|RandomFloatinRange 0.2 0.4)))
    (:then_2
      (Components|Timeline|SetPlaybackPosition _rotation_tl (Math|Random|RandomFloatinRange 0.0 (Components|Timeline|GetTimelineLength _rotation_tl)) false true)
      (Components|Timeline|SetPlayRate (Variables|Default|GetRotation%20TL) (* (Math|Random|RandomFloatinRange 0.1 0.2) (select (Math|Random|RandomBool) -1.0 1.0))))))

(fn ConstructionScript
  (bind _heal_amount (Variables|Default|GetHeal%20Amount))
  (bind _returnvalue (Math|Float|MapRangeUnclamped _heal_amount 0.0 255.0 0.0 1.0))
  (bind _material (Utilities|MakeDynamicMaterial(Static) (Variables|Default|GetBottle)))
  (Rendering|Material|SetScalarParameterValue _material "Full" _returnvalue :!class /Script/Engine.MaterialInstanceDynamic)
  (Rendering|Components|Light|SetIntensity (Variables|Default|GetPointLight) (* _returnvalue 5e+01)))