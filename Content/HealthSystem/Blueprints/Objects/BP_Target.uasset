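; BP_Target is a target actor in the health system that displays its health through a health bar widget and a text label.
; On BeginPlay it caches the local first-person character and passes its ACHealth component to the WB_HealthBar widget.
; The component's HealthUpdated event rewrites the text with the rounded current health.
; Every Tick, FaceCamera is called on both displays with the cached player.
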(event HealthUpdated(AC_Health)
  (Rendering|Components|TextRender|SetText (Variables|Default|GetTextRender) (Utilities|Text|ToText(Float) (Variables|/Game/HealthSystem/Blueprints/ActorComponent/AC_Health.AC_Health_C|GetCurrent%20Health (Variables|Default|GetAC_Health)) "HalfToEven" false true 1 324 0 0)))

(event EventTick
  (params (DeltaSeconds :type Float%20%28single-precision%29))
  (Utilities|FaceCamera (Variables|Default|GetTextRender) (Variables|Default|GetLocal%20Player))
  (Utilities|FaceCamera (Variables|Default|GetHealth%20Bar) (Variables|Default|GetLocal%20Player)))

(event EventBeginPlay
  (bind _asbp_first_person_character (Utilities|Casting|CastToBP_FirstPersonCharacter (Pawn|GetControlledPawn (Game|GetPlayerController 0))))
  (Variables|Default|SetLocal%20Player _asbp_first_person_character)
  (bind _aswb_health_bar (Utilities|Casting|CastToWB_HealthBar (UserInterface|GetWidget (Variables|Default|GetHealth%20Bar))))
  (Variables|/Game/HealthSystem/Blueprints/ActorComponent/WB_HealthBar.WB_HealthBar_C|SetAC%20Health _aswb_health_bar (Variables|Default|GetAC_Health)))

(fn ConstructionScript)