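; BP_Tree is a tree actor that visually grows and shrinks with the health held in its AC_Health component.
; UpdateTree, run on health updates and in construction, remaps the health ratio through clamped ranges to scale the large mesh, small mesh and capsule scene separately.
; Health increases and decreases trigger HealParticles above the tree, flagged as damage for losses.
; The construction script also randomizes each mesh's yaw for variety.
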(event HealthUpdated(AC_Health)
  (CallFunction|UpdateTree))

(event HealthIncreased(AC_Health)
  (Utilities|HealParticles (Variables|Default|GetDefaultSceneRoot) 2.5e+02 2.5 false))

(event HealthDecreased(AC_Health)
  (Utilities|HealParticles (Variables|Default|GetDefaultSceneRoot) 2.5e+02 2.5 true))

(event Custom|Update%20Tree
  (bind _ac_health (Variables|Default|GetAC_Health))
  (bind _ac_health_2 (Variables|Default|GetAC_Health))
  (bind _ac_health_3 (Variables|Default|GetAC_Health))
  (bind _ac_health_4 (Variables|Default|GetAC_Health))
  (bind _current_health (Variables|/Game/HealthSystem/Blueprints/AC_HealthSystem.AC_HealthSystem_C|GetCurrent%20Health _ac_health))
  (bind _max_health (Variables|/Game/HealthSystem/Blueprints/AC_HealthSystem.AC_HealthSystem_C|GetMax%20Health _ac_health_2))
  (bind _max_health_2 (Variables|/Game/HealthSystem/Blueprints/AC_HealthSystem.AC_HealthSystem_C|GetMax%20Health _ac_health))
  (bind _current_health_2 (Variables|/Game/HealthSystem/Blueprints/AC_HealthSystem.AC_HealthSystem_C|GetCurrent%20Health _ac_health_2))
  (bind _returnvalue (/ _current_health _max_health_2))
  (bind _returnvalue_2 (/ _current_health_2 _max_health))
  (bind _returnvalue_3 (Math|Float|MapRangeClamped _returnvalue 0.0 1.0 1.0 2.0))
  (bind _returnvalue_4 (Math|Float|MapRangeClamped _returnvalue_2 0.2 1.0 0.0 1.0))
  (Utilities|FlowControl|Sequence
    (:then_0
      (Transformation|SetRelativeScale3D (Variables|Default|GetLargeTreeMesh) (Math|Vector|MakeVector _returnvalue_4 _returnvalue_4 (Math|Float|MapRangeClamped _returnvalue_2 0.2 1.0 0.2 1.0))))
    (:then_1
      (Transformation|SetRelativeScale3D (Variables|Default|GetSmallTreeMesh) (Math|Conversions|ToVector(Float) (Math|Float|MapRangeClamped (/ (Variables|/Game/HealthSystem/Blueprints/AC_HealthSystem.AC_HealthSystem_C|GetCurrent%20Health _ac_health_4) (Variables|/Game/HealthSystem/Blueprints/AC_HealthSystem.AC_HealthSystem_C|GetMax%20Health _ac_health_4)) 0.0 1.0 0.1 1.0))))
    (:then_2
      (Transformation|SetRelativeScale3D (Variables|Default|GetCapsule%20Scene) (Math|Vector|MakeVector _returnvalue_3 _returnvalue_3 (Math|Float|MapRangeClamped (/ (Variables|/Game/HealthSystem/Blueprints/AC_HealthSystem.AC_HealthSystem_C|GetCurrent%20Health _ac_health_3) (Variables|/Game/HealthSystem/Blueprints/AC_HealthSystem.AC_HealthSystem_C|GetMax%20Health _ac_health_3)) 0.0 1.0 0.5 7.0))))))

(event EventBeginPlay)

(event Collision|EventActorBeginOverlap
  (params (OtherActor :type Actor%20Object%20Reference)))

(event EventTick
  (params (DeltaSeconds :type Float%20%28single-precision%29)))

(fn ConstructionScript
  (Transformation|SetRelativeRotation (Variables|Default|GetLargeTreeMesh) (Math|Rotator|MakeRotator 0.0 0.0 (Math|Random|RandomFloatinRange 0.0 3.6e+02)) false false)
  (Transformation|SetRelativeRotation (Variables|Default|GetSmallTreeMesh) (Math|Rotator|MakeRotator 0.0 0.0 (Math|Random|RandomFloatinRange 0.0 3.6e+02)) false false)
  (CallFunction|UpdateTree))