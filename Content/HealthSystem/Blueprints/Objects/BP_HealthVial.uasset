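; BP_HealthVial is a health vial pickup that, on overlap, adds itself to the actor's AC_Health component if potion collection is allowed, then destroys itself.
; The Empty flag is passed to AddVial, and in construction it darkens the vial material and removes the point light.
; Bob and wobble timelines drive the Scene's height and pitch, with randomised start positions, yaw and wobble rate to vary each instance.
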(event OnComponentBeginOverlap(Collision)
  (params (OverlappedComponent :type Primitive%20Component%20Object%20Reference) (OtherActor :type Actor%20Object%20Reference) (OtherComp :type Primitive%20Component%20Object%20Reference) (OtherBodyIndex :type Integer) (bFromSweep :type Boolean) (SweepResult :type Hit%20Result%20Structure%20%28by%20ref%29))
  (bind _returnvalue (Actor|GetComponentbyClass OtherActor "/Game/HealthSystem/Blueprints/AC_Health.AC_Health_C"))
  (Utilities|IsValid _returnvalue
    (:Is%20Valid
      (if (Variables|/Game/HealthSystem/Blueprints/AC_Health.AC_Health_C|GetCan%20collect%20Potions _returnvalue)
        (Default|AddVial _returnvalue (Variables|Default|GetEmpty))
        (Actor|DestroyActor)))))

(event EventBeginPlay
  (bind _bob_tl (Variables|Default|GetBob%20TL))
  (bind _wobble_tl (Variables|Default|GetWobble%20TL))
  (Components|Timeline|SetPlaybackPosition _bob_tl (Math|Random|RandomFloatinRange 0.0 (Components|Timeline|GetTimelineLength _bob_tl)) false true)
  (Variables|Default|SetStarting%20Rot (Math|Random|RandomFloatinRange 0.0 3.6e+02))
  (Components|Timeline|SetPlaybackPosition _wobble_tl (Math|Random|RandomFloatinRange 0.0 (Components|Timeline|GetTimelineLength _wobble_tl)) false true)
  (Components|Timeline|SetPlayRate (Variables|Default|GetWobble%20TL) (Math|Random|RandomFloatinRange 0.5 0.75)))

(fn ConstructionScript
  (bind _material (Utilities|MakeDynamicMaterial(Static) (Variables|Default|GetVial)))
  (if (Variables|Default|GetEmpty)
    (Rendering|Material|SetScalarParameterValue _material "Emissive" 0.0 :!class /Script/Engine.MaterialInstanceDynamic)
    (Rendering|Material|SetVectorParameterValue _material "Base Colour" "(R=0.100000,G=0.100000,B=0.100000,A=1.000000)" :!class /Script/Engine.MaterialInstanceDynamic)
    (Components|DestroyComponent (Variables|Default|GetPointLight))))