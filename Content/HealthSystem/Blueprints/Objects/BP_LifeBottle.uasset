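; BP_LifeBottle is a world pickup that adds a bottle with a set Fullness to the overlapping actor's AC_HealthSystem, if it can collect.
; The construction script drives the glass material and point light intensity from Fullness.
; Timelines animate bobbing, wobble and spin at randomized phases and rates, while a spawn timeline scales it and enables collision when finished.
; On collection it shows popup text to the first-person character, shrinks and destroys itself.
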(event OnComponentBeginOverlap(Collision)
  (params (OverlappedComponent :type Primitive%20Component%20Object%20Reference) (OtherActor :type Actor%20Object%20Reference) (OtherComp :type Primitive%20Component%20Object%20Reference) (OtherBodyIndex :type Integer) (bFromSweep :type Boolean) (SweepResult :type Hit%20Result%20Structure%20%28by%20ref%29))
  (bind _returnvalue (Actor|GetComponentbyClass OtherActor "/Game/HealthSystem/Blueprints/AC_HealthSystem.AC_HealthSystem_C"))
  (Utilities|IsValid _returnvalue
    (:Is%20Valid
      (if (Variables|/Game/HealthSystem/Blueprints/AC_HealthSystem.AC_HealthSystem_C|GetCan%20collect%20Life%20Bottles _returnvalue)
        (Utilities|FlowControl|DoOnce false
          (:Completed
            (Default|AddBottle _returnvalue (Variables|Default|GetFullness))
            (Utilities|FlowControl|Sequence
              (:then_0
                (bind _asbp_first_person_character (Utilities|Casting|CastToBP_FirstPersonCharacter OtherActor))
                (Default|PopupText _asbp_first_person_character "Found Life Bottle"))
              (:then_1
                (Utilities|String|Reverse (Variables|Default|GetSpawn%20TL))
                (Utilities|FlowControl|Delay 0.2)
                (Actor|DestroyActor)))))))))

(event EventBeginPlay
  (bind _wobble_tl (Variables|Default|GetWobble%20TL))
  (bind _rotation_tl (Variables|Default|GetRotation%20TL))
  (bind _bob_tl (Variables|Default|GetBob%20TL))
  (Utilities|FlowControl|Sequence
    (:then_0
      (Components|Timeline|SetPlaybackPosition _bob_tl (Math|Random|RandomFloatinRange 0.0 (Components|Timeline|GetTimelineLength _bob_tl)) false true)
      (Components|Timeline|SetPlayRate (Variables|Default|GetBob%20TL) (Math|Random|RandomFloatinRange 0.2 0.4)))
    (:then_1
      (Components|Timeline|SetPlaybackPosition _wobble_tl (Math|Random|RandomFloatinRange 0.0 (Components|Timeline|GetTimelineLength _wobble_tl)) false true)
      (Components|Timeline|SetPlayRate (Variables|Default|GetWobble%20TL) (Math|Random|RandomFloatinRange 0.2 0.4)))
    (:then_2
      (Components|Timeline|SetPlaybackPosition _rotation_tl (Math|Random|RandomFloatinRange 0.0 (Components|Timeline|GetTimelineLength _rotation_tl)) false true)
      (Components|Timeline|SetPlayRate (Variables|Default|GetRotation%20TL) (* (Math|Random|RandomFloatinRange 0.1 0.2) (select (Math|Random|RandomBool) -1.0 1.0))))))

(fn ConstructionScript
  (bind _material (Utilities|MakeDynamicMaterial(Static) (Variables|Default|GetBottle)))
  (Rendering|Material|SetScalarParameterValue _material "Full" (Variables|Default|GetFullness) :!class /Script/Engine.MaterialInstanceDynamic)
  (Rendering|Components|Light|SetIntensity (Variables|Default|GetPointLight) (Math|Float|MapRangeUnclamped (Variables|Default|GetFullness) 0.0 1.0 0.0 1e+02)))