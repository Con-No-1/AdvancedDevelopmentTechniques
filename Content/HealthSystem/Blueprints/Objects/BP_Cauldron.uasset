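; Cauldron actor that stores energy in its health component and converts it into BP_EnergyVial pickups, damaging itself to fill each vial.
; SpawnType sets vial size and trigger: looping timer, reaching full charge, storage only, or a retriggerable-delay debounce once healing stops.
; A timeline arcs each vial to a random nearby point.
; Stored health drives the light's intensity and feeds a health bar widget that faces the player.
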(event HealthIncreased(AC_Health)
  (if (and (>= (Variables|/Game/HealthSystem/Blueprints/AC_HealthSystem.AC_HealthSystem_C|GetCurrent%20Health (Variables|Default|GetAC_Health)) 225.0) (Utilities|Enum|Equal(Enum) (Variables|Default|GetSpawn%20Type) "NewEnumerator0"))
    (Utilities|DoOncePerX 1.0)
    (Utilities|FlowControl|DelayUntilNextTick)
    (if (>= (Variables|/Game/HealthSystem/Blueprints/AC_HealthSystem.AC_HealthSystem_C|GetCurrent%20Health (Variables|Default|GetAC_Health)) 5.0)
      (CallFunction|SpawnVial))))

(event HealthUpdated(AC_Health)
  (Rendering|Components|Light|SetIntensity (Variables|Default|GetPointLight) (Math|Float|MapRangeClamped (Variables|/Game/HealthSystem/Blueprints/AC_HealthSystem.AC_HealthSystem_C|GetCurrent%20Health (Variables|Default|GetAC_Health)) 0.0 225.0 0.0 2.5e+03))
  (if (Utilities|Enum|Equal(Enum) (Variables|Default|GetSpawn%20Type) "NewEnumerator4")
    (Utilities|FlowControl|RetriggerableDelay 0.1)
    (if (> (Variables|/Game/HealthSystem/Blueprints/AC_HealthSystem.AC_HealthSystem_C|GetCurrent%20Health (Variables|Default|GetAC_Health)) 0.0)
      (CallFunction|SpawnVial))))

(event Custom|Spawn%20Energy%20Vial
  (bind _spawn_type (Variables|Default|GetSpawn%20Type))
  (if (Math|Boolean|ORBoolean (Utilities|Enum|Equal(Enum) _spawn_type "NewEnumerator1") (Utilities|Enum|Equal(Enum) _spawn_type "NewEnumerator2") (and (>= (Variables|/Game/HealthSystem/Blueprints/AC_HealthSystem.AC_HealthSystem_C|GetCurrent%20Health (Variables|Default|GetAC_Health)) 225.0) (Utilities|Enum|Equal(Enum) (Variables|Default|GetSpawn%20Type) "NewEnumerator0")))
    (if (>= (Variables|/Game/HealthSystem/Blueprints/AC_HealthSystem.AC_HealthSystem_C|GetCurrent%20Health (Variables|Default|GetAC_Health)) 5.0)
      (CallFunction|SpawnVial))))

(event Custom|Spawn%20Vial
  (Variables|Default|SetTarget%20Spawn (+ (Transformation|GetActorLocation) (* (Math|Rotator|MakeRotator 0.0 0.0 (Math|Random|RandomFloatinRange 0.0 3.6e+02)) (Math|Random|RandomFloatinRange 1e+02 1.5e+02))))
  (bind _returnvalue (CallFunction|CalcEnergyVialAmount))
  (bind _damage_done (Default|Damage (Variables|Default|GetAC_Health) _returnvalue "NewEnumerator0"))
  (bind _returnvalue_2 (Game|SpawnActorfromClass "/Game/HealthSystem/Blueprints/Objects/BP_EnergyVial.BP_EnergyVial_C" (Math|Transform|MakeTransform (Transformation|GetActorLocation) "0, 0, 0" "1.000000,1.000000,1.000000") "Undefined" "MultiplyWithRoot" 0 _damage_done 0))
  (bind (_direction _lerp __z) (Timeline|Spawn%20TL PlayFromStart)
    (:Update
      (Utilities|IsValid _returnvalue_2
        (:Is%20Valid
          (Transformation|SetActorLocation _returnvalue_2 (Math|Vector|MakeVector (.x (Math|Vector|Lerp(Vector) (+ (Transformation|GetActorLocation) "0.000000,0.000000,25.000000") (Variables|Default|GetTarget%20Spawn) _lerp)) (.y (Math|Vector|Lerp(Vector) (+ (Transformation|GetActorLocation) "0.000000,0.000000,25.000000") (Variables|Default|GetTarget%20Spawn) _lerp)) (+ (.z (Math|Vector|Lerp(Vector) (+ (Transformation|GetActorLocation) "0.000000,0.000000,25.000000") (Variables|Default|GetTarget%20Spawn) _lerp)) __z)) false false))))))

(event EventBeginPlay
  (Utilities|FlowControl|Sequence
    (:then_0
      (bind _asbp_first_person_character (Utilities|Casting|CastToBP_FirstPersonCharacter (Game|Player|GetPlayerPawn 0)))
      (Variables|Default|SetPlayer _asbp_first_person_character)
      (bind _aswb_health_bar (Utilities|Casting|CastToWB_HealthBar (UserInterface|GetWidget (Variables|Default|GetHealth%20Bar))))
      (Variables|/Game/HealthSystem/Widgets+UI/WB_HealthBar.WB_HealthBar_C|SetAC%20Health _aswb_health_bar (Variables|Default|GetAC_Health)))
    (:then_1
      (if (Utilities|Enum|NotEqual(Enum) (Variables|Default|GetSpawn%20Type) "NewEnumerator4")
        (Utilities|Time|SetTimerbyEvent (delegate Custom|Spawn%20Energy%20Vial) (Variables|Default|GetSpawn%20Rate) true true)))))

(event EventTick
  (params (DeltaSeconds :type Float%20%28single-precision%29))
  (Utilities|FaceCamera (Variables|Default|GetHealth%20Bar) (Variables|Default|GetPlayer)))

(fn ConstructionScript)

(fn CalcEnergyVialAmount
  (bind _ac_health (Variables|Default|GetAC_Health))
  (bind _ac_health_2 (Variables|Default|GetAC_Health))
  (bind _current_health (Variables|/Game/HealthSystem/Blueprints/AC_HealthSystem.AC_HealthSystem_C|GetCurrent%20Health _ac_health_2))
  (bind _current_health_2 (Variables|/Game/HealthSystem/Blueprints/AC_HealthSystem.AC_HealthSystem_C|GetCurrent%20Health _ac_health))
  (bind _returnvalue (Math|Float|Clamp(Float) _current_health 0.0 225.0))
  (bind _returnvalue_2 (Math|Random|RandomFloatinRange 5.0 _returnvalue))
  (return (Math|Float|Clamp(Float) (Utilities|Select :Index (Variables|Default|GetSpawn%20Type) :NewEnumerator1 (select (< (- (Variables|/Game/HealthSystem/Blueprints/AC_HealthSystem.AC_HealthSystem_C|GetCurrent%20Health (Variables|Default|GetAC_Health)) _returnvalue_2) 5.0) (+ _returnvalue_2 5.0) _returnvalue_2) :NewEnumerator2 _current_health_2 :NewEnumerator0 225.0 :NewEnumerator3 0.0 :NewEnumerator4 _current_health_2) 0.0 (Variables|/Game/HealthSystem/Blueprints/AC_HealthSystem.AC_HealthSystem_C|GetCurrent%20Health (Variables|Default|GetAC_Health)))))