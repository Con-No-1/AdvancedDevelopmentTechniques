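; Fountain actor that, depending on its Heal flag, either heals or damages actors with an AC_HealthSystem inside its sphere.
; Each Tick applies a frame-scaled rate, with distance falloff only for the local player.
; Its own health component acts as the reservoir: healing drains it until empty, while damage dealt fills it from zero.
; That reservoir drives the camera-facing text and Niagara spawn rate, with the effect asset chosen in the construction script.
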(event HealthUpdated(AC_Health)
  (CallFunction|UpdateHealthUI))

(event Custom|Update%20Health%20UI
  (Utilities|FlowControl|Sequence
    (:then_0
      (Rendering|Components|TextRender|SetText (Variables|Default|GetHealth) (Utilities|Text|FormatText "{hp} 
{HPS}: {hps}" (Utilities|Text|ToText(Float) (Variables|/Game/HealthSystem/Blueprints/AC_HealthSystem.AC_HealthSystem_C|GetCurrent%20Health (Variables|Default|GetAC_Health)) "HalfToEven" false true 1 324 0 0) (select (Variables|Default|GetHeal) "HPS" "DPS") (Variables|Default|GetHP/DMG/s))))
    (:then_1
      (Effects|Components|ParticleSystem|SetFloatParameter (Variables|Default|GetNS_HealthFountain) "SpawnRate" (Math|Float|MapRangeClamped (Variables|/Game/HealthSystem/Blueprints/AC_HealthSystem.AC_HealthSystem_C|GetCurrent%20Health (Variables|Default|GetAC_Health)) 0.0 6e+02 (select (Variables|Default|GetHeal) 0.0 5e+01) 5e+01)))
    (:then_2
      (if (and (<= (Variables|/Game/HealthSystem/Blueprints/AC_HealthSystem.AC_HealthSystem_C|GetCurrent%20Health (Variables|Default|GetAC_Health)) 0.0) (Variables|Default|GetHeal))
        (Rendering|Components|TextRender|SetText (Variables|Default|GetHealth) (Utilities|Text|FormatText ""))))))

(event EventTick
  (params (DeltaSeconds :type Float%20%28single-precision%29))
  (Variables|Default|SetDelta%20Seconds DeltaSeconds)
  (Utilities|FlowControl|Sequence
    (:then_0
      (if (or (> (Variables|/Game/HealthSystem/Blueprints/AC_HealthSystem.AC_HealthSystem_C|GetCurrent%20Health (Variables|Default|GetAC_Health)) 0.0) (not (Variables|Default|GetHeal)))
        (for _array_element (Collision|GetOverlappingActors (Variables|Default|GetSphere) 0 :!class /Script/Engine.PrimitiveComponent)
          (Utilities|IsValid (Actor|GetComponentbyClass _array_element "/Game/HealthSystem/Blueprints/AC_HealthSystem.AC_HealthSystem_C")
            (:Is%20Valid
              (Variables|Default|SetTarget%20Actor _array_element)
              (Variables|Default|SetTarget%20AC_Health (Actor|GetComponentbyClass _array_element "/Game/HealthSystem/Blueprints/AC_HealthSystem.AC_HealthSystem_C"))
              (if (Variables|Default|GetHeal)
                (bind _heal (CallFunction|CalcHealAmount))
                (bind _heal_done (Default|Heal (Variables|Default|GetTarget%20AC_Health) _heal))
                (Default|Damage (Variables|Default|GetAC_Health) _heal_done)
                (else
                  (bind _damage (CallFunction|CalcDamageAmount))
                  (bind _damage_done (Default|Damage (Variables|Default|GetTarget%20AC_Health) _damage))
                  (Default|Heal (Variables|Default|GetAC_Health) _damage_done))))))))
    (:then_1
      (Utilities|FaceCamera (Variables|Default|GetHealth) (Variables|Default|GetLocal%20Player)))))

(event EventBeginPlay
  (bind _asbp_first_person_character (Utilities|Casting|CastToBP_FirstPersonCharacter (Pawn|GetControlledPawn (Game|GetPlayerController 0))))
  (Variables|Default|SetLocal%20Player _asbp_first_person_character))

(fn ConstructionScript
  (Utilities|FlowControl|Sequence
    (:then_0
      (CallFunction|UpdateHealthUI)
      (Class|NiagaraComponent|SetAsset (Variables|Default|GetNS_HealthFountain) (select (Variables|Default|GetHeal) "/Game/HealthSystem/VFX/NS_HealthFountain.NS_HealthFountain" "/Game/HealthSystem/VFX/NS_DamageFountain.NS_DamageFountain") true))
    (:then_1
      (if (not (Variables|Default|GetHeal))
        (Variables|/Game/HealthSystem/Blueprints/AC_HealthSystem.AC_HealthSystem_C|SetCurrent%20Health (Variables|Default|GetAC_Health) 0.0)))))

(fn OnRepRemainingHealth)

(fn CalcHealAmount
  (return (Math|Float|Clamp(Float) (* (Variables|Default|GetHP/DMG/s) (Variables|Default|GetDelta%20Seconds) (CallFunction|DistanceMulti)) 0.0 (Variables|/Game/HealthSystem/Blueprints/AC_HealthSystem.AC_HealthSystem_C|GetCurrent%20Health (Variables|Default|GetAC_Health)))))

(fn CalcDamageAmount
  (return (* (Variables|Default|GetHP/DMG/s) (Variables|Default|GetDelta%20Seconds) (CallFunction|DistanceMulti))))

(fn DistanceMulti
  (bind _sphere (Variables|Default|GetSphere))
  (bind _returnvalue (Components|Sphere|GetScaledSphereRadius _sphere))
  (if (== (Variables|Default|GetLocal%20Player) (Variables|Default|GetTarget%20Actor))
    (return (Math|Float|MapRangeClamped (Math|Vector|Distance2D(Vector) (Transformation|GetActorLocation) (Transformation|GetActorLocation (Variables|Default|GetTarget%20Actor))) _returnvalue (/ _returnvalue 2.0) 0.0 1.0))
    (else
      (return 1.0))))