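; BP_TargetDummy is a physics-driven target dummy with an AC_Health component and a camera-facing health bar widget.
; Health and bottle updates drive a dynamic material's Health ratio and briefly flash its emissive.
; Death hides the bar and zeroes the mesh's center-of-mass offset, while revival shows it and lowers the center of mass like a roly-poly toy.
; Both events also apply a random force to the mesh.
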(event Revived(AC_Health)
  (bind _returnvalue (Math|Random|RandomFloatinRange 5e+05 1e+06))
  (Rendering|SetVisibility (Variables|Default|GetHealth%20Bar) true true)
  (Class|PrimitiveComponent|SetCenterOfMass (Variables|Default|GetStatic%20Mesh) "0.000000,0.000000,-90.000000" "None")
  (Physics|AddForce (Variables|Default|GetStatic%20Mesh) (Math|Vector|MakeVector _returnvalue _returnvalue _returnvalue) "None" false))

(event HealthUpdated(AC_Health)
  (bind _ac_health (Variables|Default|GetAC_Health))
  (Rendering|Material|SetScalarParameterValue (Variables|Default|GetMaterial) "Health" (/ (Variables|/Game/HealthSystem/Blueprints/AC_Health.AC_Health_C|GetCurrent%20Health _ac_health) (Variables|/Game/HealthSystem/Blueprints/AC_Health.AC_Health_C|GetMax%20Health _ac_health)) :!class /Script/Engine.MaterialInstanceDynamic)
  (Rendering|Material|SetScalarParameterValue (Variables|Default|GetMaterial) "Emissive" 0.25 :!class /Script/Engine.MaterialInstanceDynamic)
  (Utilities|FlowControl|RetriggerableDelay 0.1)
  (Rendering|Material|SetScalarParameterValue (Variables|Default|GetMaterial) "Emissive" 0.0 :!class /Script/Engine.MaterialInstanceDynamic))

(event Death(AC_Health)
  (bind _returnvalue (Math|Random|RandomFloatinRange 5e+05 1e+06))
  (Rendering|SetVisibility (Variables|Default|GetHealth%20Bar) false true)
  (Class|PrimitiveComponent|SetCenterOfMass (Variables|Default|GetStatic%20Mesh) "0, 0, 0" "None")
  (Physics|AddForce (Variables|Default|GetStatic%20Mesh) (Math|Vector|MakeVector _returnvalue _returnvalue _returnvalue) "None" false))

(event Bottle%Updated(AC_Health)
  (bind _ac_health (Variables|Default|GetAC_Health))
  (Rendering|Material|SetScalarParameterValue (Variables|Default|GetMaterial) "Health" (/ (Variables|/Game/HealthSystem/Blueprints/AC_Health.AC_Health_C|GetCurrent%20Health _ac_health) (Variables|/Game/HealthSystem/Blueprints/AC_Health.AC_Health_C|GetMax%20Health _ac_health)) :!class /Script/Engine.MaterialInstanceDynamic)
  (Rendering|Material|SetScalarParameterValue (Variables|Default|GetMaterial) "Emissive" 0.25 :!class /Script/Engine.MaterialInstanceDynamic)
  (Utilities|FlowControl|RetriggerableDelay 0.1)
  (Rendering|Material|SetScalarParameterValue (Variables|Default|GetMaterial) "Emissive" 0.0 :!class /Script/Engine.MaterialInstanceDynamic))

(event EventTick
  (params (DeltaSeconds :type Float%20%28single-precision%29))
  (Utilities|FaceCamera (Variables|Default|GetHealth%20Bar) (Variables|Default|GetLocal%20Player)))

(event EventBeginPlay
  (bind _asbp_first_person_character (Utilities|Casting|CastToBP_FirstPersonCharacter (Pawn|GetControlledPawn (Game|GetPlayerController 0))))
  (Variables|Default|SetLocal%20Player _asbp_first_person_character)
  (bind _aswb_health_bar (Utilities|Casting|CastToWB_HealthBar (UserInterface|GetWidget (Variables|Default|GetHealth%20Bar))))
  (Variables|/Game/HealthSystem/Widgets+UI/WB_HealthBar.WB_HealthBar_C|SetAC%20Health _aswb_health_bar (Variables|Default|GetAC_Health)))

(fn ConstructionScript
  (bind _material (Utilities|MakeDynamicMaterial(Static) (Variables|Default|GetStatic%20Mesh)))
  (Variables|Default|SetMaterial _material))